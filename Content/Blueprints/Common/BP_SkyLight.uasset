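; BP_SkyLight is a time-driven sky lighting actor that sets light intensity, rotation and color from curves.
; Update reads LightCurve for intensity (X) and actor rotation (Y, Z), and ColorCurve for a color shared by all lights.
; Four AmbientLight components, named by 90-degree steps, follow the main light's intensity, scaled by Ambient and clamped.
; The construction script also calls Update, applying the current Time at construction.
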(event Custom|Update
  (params (Time :type Float%20%28single-precision%29))
  (bind _lightcurve (Variables|Curves|GetLightCurve))
  (bind _returnvalue (Math|Curves|GetVectorValue _lightcurve Time))
  (Variables|Properties|SetLightIntensity (.x _returnvalue))
  (bind _output_get (Variables|Properties|SetLightRotation (Math|Rotator|MakeRotator 0.0 (.y _returnvalue) (.z _returnvalue))))
  (Transformation|SetActorRotation _output_get)
  (Rendering|Components|Light|SetIntensity)
  (Maerial|SetColor Time))

(fn ConstructionScript
  (CallFunction|Update (Variables|Options|GetTime)))