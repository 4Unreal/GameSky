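; Moon component for a sky system that drives the owning moon actor and the sky material's moon from time of day and phase.
; Update offsets time by phase through wrapping rotator math to get lunar time, which samples a curve for rotation.
; The owner takes that rotation directly, with intensity and ambient mapped from sun height.
; The material receives an interpolated direction plus brightness, phase, disc orientation and pitch-based scale.
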(fn GetMoonRotation
  (params (Time :type Float%20%28single-precision%29) (MoonPhase :type Float%20%28single-precision%29) (RotationCurve :type Curve%20Vector%20Object%20Reference))
  (bind _returnvalue (Math|Float|MapRangeUnclamped Time 0.0 24.0 -1.8e+02 1.8e+02))
  (bind _returnvalue_2 (Math|Float|MapRangeClamped MoonPhase 0.0 1.0 1.8e+02 -1.8e+02))
  (bind _returnvalue_3 (Math|Rotator|MakeRotator _returnvalue 0.0 0.0))
  (bind _returnvalue_4 (Math|Rotator|CombineRotators _returnvalue_3 (Math|Rotator|MakeRotator _returnvalue_2 0.0 0.0)))
  (bind _returnvalue_5 (Math|Float|MapRangeClamped (.roll _returnvalue_4) -1.8e+02 1.8e+02 0.0 24.0))
  (bind _returnvalue_6 (Math|Curves|GetVectorValue RotationCurve _returnvalue_5))
  (return (Math|Rotator|CombineRotators (Math|Rotator|MakeRotator 0.0 (.y _returnvalue_6) (.z _returnvalue_6)) (Math|Rotator|MakeRotator 0.0 -8.0 0.0)) _returnvalue_5))

(fn SetDirection
  (params (Rotation :type Rotator) (InterpSpeed :type Float%20%28single-precision%29))
  (bind _output_get (Variables|Default|SetDirection (Math|Interpolation|VInterpTo (Variables|Default|GetDirection) (Math|Rotator|GetRotationXVector Rotation) (Utilities|Time|GetWorldDeltaSeconds) InterpSpeed)))
  (return (Math|Conversions|ToLinearColor(Vector) _output_get)))

(fn GetOrientation
  (bind _direction (Variables|Default|GetDirection))
  (bind _returnvalue (Math|Conversions|RotationFromXVector _direction))
  (return (select (> (.yaw _returnvalue) 0.0) (Math|Float|MapRangeUnclamped (.yaw _returnvalue) 9e+01 1.8e+02 0.22 0.32) (Math|Float|MapRangeUnclamped (.yaw _returnvalue) -1.8e+02 -9e+01 0.32 0.22))))

(fn Update
  (params (Time :type Float%20%28single-precision%29) (MoonPhase :type Float%20%28single-precision%29) (RotationCurve :type Curve%20Vector%20Object%20Reference) (SkyMaterial :type Material%20Instance%20Dynamic%20Object%20Reference) (SunHeight :type Float%20%28single-precision%29) (InterpSpeed :type Float%20%28single-precision%29))
  (bind (_returnvalue _lunartime) (CallFunction|GetMoonRotation Time MoonPhase RotationCurve))
  (bind _output_get (Variables|Default|SetRotation _returnvalue))
  (|UpdateLightActor _output_get _lunartime SunHeight)
  (bind _returnvalue_2 (CallFunction|SetDirection _output_get InterpSpeed))
  (Rendering|Material|SetVectorParameterValue SkyMaterial "Moon Direction" _returnvalue_2 :!class /Script/Engine.MaterialInstanceDynamic)
  (Rendering|Material|SetScalarParameterValue SkyMaterial "Moon Brightness" (Utilities|GetMoonBrightness MoonPhase SunHeight) :!class /Script/Engine.MaterialInstanceDynamic)
  (Rendering|Material|SetScalarParameterValue SkyMaterial "Moon Phase" MoonPhase :!class /Script/Engine.MaterialInstanceDynamic)
  (bind _returnvalue_3 (CallFunction|GetOrientation))
  (Rendering|Material|SetScalarParameterValue SkyMaterial "Moon Rotation" _returnvalue_3 :!class /Script/Engine.MaterialInstanceDynamic)
  (bind _returnvalue_4 (CallFunction|MapHeightRange 0.1 0.2))
  (Rendering|Material|SetScalarParameterValue SkyMaterial "Moon Scale" _returnvalue_4 :!class /Script/Engine.MaterialInstanceDynamic)
  (return))

(fn MapHeightRange
  (params (OutRangeA :type Float%20%28single-precision%29) (OutRangeB :type Float%20%28single-precision%29))
  (return (Math|Float|MapRangeClamped (.pitch (Variables|Default|GetRotation)) -4e+01 0.0 OutRangeA OutRangeB)))