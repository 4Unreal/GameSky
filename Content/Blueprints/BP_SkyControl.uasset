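; BP_SkyControl is a manager actor that drives the sky and time of day from a single Time value.
; Update pushes Time to the first BP_SkySun and to the first BP_SkySphere, which also receives MoonPhase.
; TimeTick stores a new Time and refreshes both.
; The construction script also runs Update and copies Time into the first BP_DayTimeClock's StartTime, each target found via GetAllActorsOfClass.
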(event Custom|Update
  (Utilities|FlowControl|Sequence
    (:then_0
      (|UpdateSun))
    (:then_1
      (|UpdateSky))))

(event EventTimeTick
  (params (Time :type Float%20%28single-precision%29))
  (Variables|Controls|SetTime Time)
  (CallFunction|Update))

(fn ConstructionScript
  (Utilities|FlowControl|Sequence
    (:then_0
      (CallFunction|Update))
    (:then_1
      (|SetClockStartTime))))