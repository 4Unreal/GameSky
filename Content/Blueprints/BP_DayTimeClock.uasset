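; Day-time clock actor that tracks a 24-hour Time value and broadcasts it to time-aware actors.
; BeginPlay seeds Time from StartTime and sets the matching position on the DayTime timeline.
; Each timeline update eases Time toward the timeline's value, converting both to roll angles so interpolation treats hours as circular.
; It then re-queries every BPI_TimeAware actor and sends each a TimeTickMessage.
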(event EventBeginPlay
  (bind _starttime (Variables|Options|GetStartTime))
  (Variables|Default|SetTime _starttime)
  (bind _time (Timeline|DayTime SetNewTime)
    (:Update
      (bind _outactors (Actor|GetAllActorswithInterface "/GameSky/Blueprints/Interfaces/BPI_TimeAware.BPI_TimeAware_C"))
      (Variables|Default|SetTime (Math|Float|MapRangeClamped (.roll (Math|Interpolation|Ease "Linear" 0.1 (Math|Rotator|MakeRotator (Math|Float|MapRangeClamped (Variables|Default|GetTime) 0.0 24.0 -1.8e+02 1.8e+02) 0.0 0.0) (Math|Rotator|MakeRotator (Math|Float|MapRangeClamped _time 0.0 24.0 -1.8e+02 1.8e+02) 0.0 0.0) true)) -1.8e+02 1.8e+02 0.0 23.999))
      (for _array_element _outactors
        (Class|BPITimeAware|TimeTick(Message) _array_element (Variables|Default|GetTime))))))

(fn ConstructionScript)